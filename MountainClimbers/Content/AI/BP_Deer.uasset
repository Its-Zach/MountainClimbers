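; BP_Deer is an AI deer that detects player vehicles and knocks them away.
; Sighting a vehicle pawn sets the "HasSeenPlayer?" blackboard key, which a retriggerable delay clears shortly after sightings stop.
; AttackBox overlap launches the vehicle mesh away from the deer by LaunchStrength, using the pawn from the sight event rather than the overlapping actor.
; Roam_Around is an empty stub.
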(event OnSeePawn(PawnSensing)
  (params (Pawn :type Pawn%20Object%20Reference))
  (bind _returnvalue (Utilities|Name|MakeLiteralName "HasSeenPlayer?"))
  (bind _self self)
  (bind _returnvalue_2 (AI|GetAIController _self))
  (bind _returnvalue_3 (AI|GetBlackboard _returnvalue_2))
  (Utilities|Casting|CastToBP_VehicleAdvPawnBase Pawn)
  (AI|Components|Blackboard|SetValueasBool _returnvalue_3 _returnvalue true)
  (Utilities|FlowControl|RetriggerableDelay 0.6)
  (AI|Components|Blackboard|SetValueasBool _returnvalue_3 _returnvalue false))

(event OnComponentBeginOverlap(AttackBox)
  (params (OverlappedComponent :type Primitive%20Component%20Object%20Reference) (OtherActor :type Actor%20Object%20Reference) (OtherComp :type Primitive%20Component%20Object%20Reference) (OtherBodyIndex :type Integer) (bFromSweep :type Boolean) (SweepResult :type Hit%20Result%20Structure%20%28by%20ref%29))
  (Development|PrintString "Hit")
  (bind _asbp_vehicle_adv_pawn_base (Utilities|Casting|CastToBP_VehicleAdvPawnBase (stale OnSeePawn(PawnSensing) Pawn)))
  (Development|PrintString "Cast")
  (Physics|AddImpulse (Variables|/Script/ChaosVehicles.WheeledVehiclePawn|GetMesh _asbp_vehicle_adv_pawn_base) (* (Math|Vector|Normalize (- (Transformation|GetActorLocation (stale OnSeePawn(PawnSensing) Pawn)) (Transformation|GetActorLocation))) (Variables|Default|GetLaunchStrength)) "None" true))

(event Custom|Roam_Around)

(event EventBeginPlay)

(fn ConstructionScript)